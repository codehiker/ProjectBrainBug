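; Enemy drop ship for the SHMUP starter that moves its mesh up and down, extending the parent's BeginPlay.
; A Parabola timeline starts on BeginPlay, and its output is remapped to a relative Z offset that moves ShipMesh with sweep enabled.
; When the timeline finishes, it restarts after a short delay, so the vertical motion repeats continuously.
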(event `self.ReceiveBeginPlay`
  ;[1 1 1] Initialization
  (`parent.ReceiveBeginPlay`)
  (`self.MoveUpAndDown`))

(event `MoveUpAndDown`
  ;[1 1 1] Parabolic movement (up and down)
  (bind (_direction _position) (`Timeline|Parabola` :!via `PlayFromStart` :!label _label)
    (:`Update`
      (`SceneComponent.K2_SetRelativeLocation` (`self.ShipMesh`) (`KismetMathLibrary.MakeVector` 0.0 0.0 (`KismetMathLibrary.MapRangeClamped` _position -1.0 1.0 -700.0 700.0)) true false))
    (:`Finished`
      (`KismetSystemLibrary.Delay` 0.2)
      (goto _label :!via `PlayFromStart`))))

(fn `UserConstructionScript`
  (`parent.UserConstructionScript`))