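; Asteroid enemy for the shmup, built on a parent enemy ship, that tumbles and splits into smaller asteroids on death.
; Construction randomizes vertical movement and speed, and uses BreakSize to pick the mesh and collision sphere radius.
; BeginPlay picks a random spin applied each tick and stores starting Health for offspring.
; DieChild recursively spawns two vertically offset copies with BreakSize reduced by one until it reaches zero.
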(event `self.ReceiveBeginPlay`
  (bind _returnvalue (`KismetMathLibrary.RandomFloatInRange` -200.0 200.0))
  ;[1 1 1] Initialization
  (`parent.ReceiveBeginPlay`)
  ;;[1 1 1] Set random values for rotation
  (set `self.X` _returnvalue)
  (set `self.Y` _returnvalue)
  (set `self.Z` _returnvalue)
  ;;[1 1 1] Set health on asteroid pieces
  (set `self.OffspringHealth` (`self.Health`)))

(event `self.ReceiveTick`
  (params (DeltaSeconds :type "Float (single-precision)"))
  ;[1 1 1] Tick
  (`parent.ReceiveTick` DeltaSeconds)
  (`self.RotateAsteroid`))

(event `RotateAsteroid`
  (bind _shipmesh (`self.ShipMesh`))
  ;[1 1 1] Randomly rotate the asteroid
  (`/Engine/EditorBlueprintResources/StandardMacros.IsValid` _shipmesh
    (:`Is Valid`
      (`SceneComponent.K2_AddLocalRotation` _shipmesh (`/Game/SHMUP_starter/Blueprints/BP_SHMUP_MacroLibrary.RotationFI` (`KismetMathLibrary.MakeRotator` (`self.X`) (`self.Y`) (`self.Z`))) false false))))

(event `self.DieChild`
  (bind (_returnvalue_x _returnvalue_y _returnvalue_z) (`KismetMathLibrary.BreakVector` (`self.K2_GetActorLocation`)))
  ;[1 1 1] Spawn smaller pieces of the asteroid
  (if (> (`self.BreakSize`) 0)
    (for _index (range 2)
      (`|SpawnActorFromClass` "BP_EnemyShip_Asteroid_C" (`KismetMathLibrary.MakeTransform` (`KismetMathLibrary.MakeVector` _returnvalue_x _returnvalue_y (+ (- _returnvalue_z 100.0) (* _index 200.0)))) "AdjustIfPossibleButAlwaysSpawn" "OverrideRootScale" null (- (`self.BreakSize`) 1) (`self.OffspringHealth`) false "NewEnumerator3" 2.0 0.0 false false 2.0 40 null))))

(fn `UserConstructionScript`
  (bind _speed (`self.Speed`))
  (`parent.UserConstructionScript`)
  ;[1 1 1] Give a random initial velocity
  (set `self.VerticalMovement` (`KismetMathLibrary.RandomFloatInRange` -1.0 1.0))
  (set `self.Speed` (`KismetMathLibrary.RandomFloatInRange` (* _speed 0.5) (* _speed 1.5)))
  ;[1 1 1] Set correct mesh based on "break size"
  (`StaticMeshComponent.SetStaticMesh` (`self.ShipMesh`) (select `int` (`self.BreakSize`) :`0` "/Game/SHMUP_starter/Meshes/SM_Asteroid3.SM_Asteroid3" :`1` "/Game/SHMUP_starter/Meshes/SM_asteroid2.SM_asteroid2" :`2` "/Game/SHMUP_starter/Meshes/SM_Asteroid1.SM_Asteroid1" :!type "StaticMesh Object Reference"))
  ;[1 1 1] Adjust sweep collision sphere based on mesh size
  (`SphereComponent.SetSphereRadius` (`self.Sphere`) (select `int` (`self.BreakSize`) :`0` 40.0 :`1` 88.0 :`2` 130.0 :!type "Float (single-precision)") true))