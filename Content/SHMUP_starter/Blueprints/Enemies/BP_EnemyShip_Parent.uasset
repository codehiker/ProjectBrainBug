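; Parent Blueprint for shoot-'em-up enemy ships that move, optionally shoot, and kill the hero on contact.
; Tick scrolls the ship along Y scaled by the hero's current speed, plus a vertical offset.
; Shooters loop delayed bullet spawns, optionally aimed at the hero.
; Hero damage flashes the material and lowers health; death runs once, calling a child hook, spawning explosion and optional pickup, and adding score.
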(event `self.ReceiveBeginPlay`
  ;[1 1 1] Initialization
  (bind _asbp_hero (cast `/Game/SHMUP_starter/Blueprints/Ship/BP_Hero` (`GameplayStatics.GetPlayerPawn` 0)))
  (set `self.HeroRef` _asbp_hero)
  (set `self.DefaultMat` (`PrimitiveComponent.GetMaterial` (`self.ShipMesh`) 0))
  (if (`self.Shooter`)
    (`KismetSystemLibrary.Delay` 3.0)
    (`self.Shoot`)))

(event `self.ReceiveTick`
  (params (DeltaSeconds :type "Float (single-precision)"))
  (bind _heroref (`self.HeroRef`))
  ;[1 1 1] Tick - move at player "speed"
  (`/Engine/EditorBlueprintResources/StandardMacros.IsValid` _heroref
    (:`Is Valid`
      (`self.K2_AddActorWorldOffset` (`KismetMathLibrary.MakeVector` 0.0 (* DeltaSeconds (`/Game/SHMUP_starter/Blueprints/Ship/BP_Hero.CurrentSpeed` _heroref) (* -1.0 (`self.Speed`))) (`self.VerticalMovement`)) true))))

(event `/Game/SHMUP_starter/Blueprints/BP_iDamageable.TakeDamage`
  (params (Aggressor :type "Actor Object Reference") (Damage :type "Float (single-precision)"))
  ;[1 1 1] Take damage
  (cast `/Game/SHMUP_starter/Blueprints/Ship/BP_Hero` Aggressor)
  (`self.Flash`)
  (bind _output_get (set `self.Health` (- (`self.Health`) Damage)))
  (if (<= _output_get 0.0)
    (`self.Die`)))

(event `Die`
  ;[1 1 1] Death
  (`/Engine/EditorBlueprintResources/StandardMacros.DoOnce` false
    (:`Completed`
      (`self.DieChild`)
      (`|SpawnActorFromClass` "/Game/SHMUP_starter/Blueprints/FX/BP_Explosion.BP_Explosion_C" (`KismetMathLibrary.MakeTransform` (`SceneComponent.K2_GetComponentLocation` (`self.ShipMesh`))) "Undefined" "OverrideRootScale" null null)
      (`GameplayStatics.PlaySoundAtLocation` (`self.DeathSound`) (`self.K2_GetActorLocation`) (struct) 1.0 1.0 0.0 null null null)
      (`/Game/SHMUP_starter/Blueprints/Ship/BP_Hero.AddScore` (`self.HeroRef`) (`self.Score`))
      (if (`self.Drop?`)
        (`|SpawnActorFromClass` "/Game/SHMUP_starter/Blueprints/Weapons/BP_PickUp.BP_PickUp_C" (`KismetMathLibrary.MakeTransform` (`SceneComponent.K2_GetComponentLocation` (`self.ShipMesh`))) "Undefined" "OverrideRootScale" null (`self.Drop`) null))
      (`self.K2_DestroyActor`))))

(event `DieChild`
  ;[1 1 1] Death
  ;;[1 1 1] Call on Child BP
)

(event `Flash`
  (bind _shipmesh (`self.ShipMesh`))
  ;[1 1 1] Damage flash
  (`PrimitiveComponent.SetMaterial` _shipmesh 0 "/Game/SHMUP_starter/Materials/MI_Hit.MI_Hit")
  (`KismetSystemLibrary.Delay` 0.2)
  (`PrimitiveComponent.SetMaterial` _shipmesh 0 (`self.DefaultMat`)))

(event `Shoot`
  (bind _firevector (`self.FireVector`))
  (bind (_returnvalue_location _returnvalue_rotation) (`KismetMathLibrary.BreakTransform` (`SceneComponent.K2_GetComponentToWorld` _firevector)))
  ;[1 1 1] Shoot projectile if enabled
  (`|SpawnActorFromClass` "/Game/SHMUP_starter/Blueprints/Weapons/BP_EnemyBullet.BP_EnemyBullet_C" (`KismetMathLibrary.MakeTransform` _returnvalue_location (select `bool` (`self.Homing?`) :`false` _returnvalue_rotation :`true` (`KismetMathLibrary.FindLookAtRotation` (`SceneComponent.K2_GetComponentLocation` _firevector) (`self.K2_GetActorLocation` (`self.HeroRef`))))) "Undefined" "OverrideRootScale" null 1.0 1000.0 false null)
  (`KismetSystemLibrary.Delay` (`self.FireRate`))
  (`self.Shoot`))

(event `self.Sphere.OnComponentBeginOverlap`
  (params (OverlappedComponent :type "PrimitiveComponent Object Reference") (OtherActor :type "Actor Object Reference") (OtherComp :type "PrimitiveComponent Object Reference") (OtherBodyIndex :type Integer) (bFromSweep :type Boolean) (SweepResult :type "HitResult Structure (by ref)"))
  ;[1 1 1] Kill player on contact
  (bind _asbp_hero (cast `/Game/SHMUP_starter/Blueprints/Ship/BP_Hero` OtherActor))
  (`/Game/SHMUP_starter/Blueprints/Ship/BP_Hero.Die` :`self` _asbp_hero))

(fn `UserConstructionScript`)