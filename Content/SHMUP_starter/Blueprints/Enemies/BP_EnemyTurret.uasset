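; BP_EnemyTurret is a shoot-'em-up enemy turret that pitches its gun toward the player hero and fires bullets on a repeating delay.
; Shots follow the fire point's rotation, or aim straight at the hero at spawn when Homing is set.
; Hero damage flashes a hit material and drains health; death calls a DieChild hook for subclasses, spawns an explosion and awards score.
; Touching its base or gun kills the hero.
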(event `self.ReceiveBeginPlay`
  ;[1 1 1] Initialization
  (bind _asbp_hero (cast `/Game/SHMUP_starter/Blueprints/Ship/BP_Hero` (`GameplayStatics.GetPlayerPawn` 0)))
  (set `self.HeroRef` _asbp_hero)
  (set `self.DefaultMat` (`PrimitiveComponent.GetMaterial` (`self.TurretGun`) 0))
  (`KismetSystemLibrary.Delay` 3.0)
  (`self.Shoot`))

(event `self.ReceiveTick`
  (params (DeltaSeconds :type "Float (single-precision)"))
  (bind _heroref (`self.HeroRef`))
  (bind _turretgun (`self.TurretGun`))
  (bind (_returnvalue_roll _returnvalue_pitch) (`KismetMathLibrary.BreakRotator` (`KismetMathLibrary.FindLookAtRotation` (`SceneComponent.K2_GetComponentLocation` _turretgun) (`self.K2_GetActorLocation` _heroref))))
  ;[1 1 1] Tick - aim turret at player
  (`/Engine/EditorBlueprintResources/StandardMacros.IsValid` _heroref
    (:`Is Valid`
      (`SceneComponent.K2_SetWorldRotation` _turretgun (`KismetMathLibrary.MakeRotator` (- _returnvalue_pitch 90.0)) false false))))

(event `/Game/SHMUP_starter/Blueprints/BP_iDamageable.TakeDamage`
  (params (Aggressor :type "Actor Object Reference") (Damage :type "Float (single-precision)"))
  ;[1 1 1] Take damage
  (cast `/Game/SHMUP_starter/Blueprints/Ship/BP_Hero` Aggressor)
  (`self.Flash`)
  (bind _output_get (set `self.Health` (- (`self.Health`) Damage)))
  (if (<= _output_get 0.0)
    (`self.Die`)))

(event `Die`
  ;[1 1 1] Die
  (`/Engine/EditorBlueprintResources/StandardMacros.DoOnce` false
    (:`Completed`
      (`self.DieChild`)
      (`|SpawnActorFromClass` "/Game/SHMUP_starter/Blueprints/FX/BP_Explosion.BP_Explosion_C" (`KismetMathLibrary.MakeTransform` (`SceneComponent.K2_GetComponentLocation` (`self.TurretGun`))) "Undefined" "OverrideRootScale" null null)
      (`GameplayStatics.PlaySoundAtLocation` (`self.DeathSound`) (`self.K2_GetActorLocation`) (struct) 1.0 1.0 0.0 null null null)
      (`/Game/SHMUP_starter/Blueprints/Ship/BP_Hero.AddScore` (`self.HeroRef`) (`self.Score`))
      (`self.K2_DestroyActor`))))

(event `DieChild`
  ;[1 1 1] Die
  ;;[1 1 1] Call on child
)

(event `Flash`
  (bind _turretgun (`self.TurretGun`))
  ;[1 1 1] Hit flash
  (`PrimitiveComponent.SetMaterial` _turretgun 0 "/Game/SHMUP_starter/Materials/MI_Hit.MI_Hit")
  (`KismetSystemLibrary.Delay` 0.2)
  (`PrimitiveComponent.SetMaterial` _turretgun 0 (`self.DefaultMat`)))

(event `Shoot`
  (bind _firevector (`self.FireVector`))
  (bind (_returnvalue_location _returnvalue_rotation) (`KismetMathLibrary.BreakTransform` (`SceneComponent.K2_GetComponentToWorld` _firevector)))
  ;[1 1 1] Shoot
  (`|SpawnActorFromClass` "/Game/SHMUP_starter/Blueprints/Weapons/BP_EnemyBullet.BP_EnemyBullet_C" (`KismetMathLibrary.MakeTransform` _returnvalue_location (select `bool` (`self.Homing?`) :`false` _returnvalue_rotation :`true` (`KismetMathLibrary.FindLookAtRotation` (`SceneComponent.K2_GetComponentLocation` _firevector) (`self.K2_GetActorLocation` (`self.HeroRef`))))) "Undefined" "OverrideRootScale" null 2.0 2000.0 false null)
  (`KismetSystemLibrary.Delay` (`self.FireRate`))
  (`self.Shoot`))

(event `self.TurretBase.OnComponentBeginOverlap`
  (params (OverlappedComponent :type "PrimitiveComponent Object Reference") (OtherActor :type "Actor Object Reference") (OtherComp :type "PrimitiveComponent Object Reference") (OtherBodyIndex :type Integer) (bFromSweep :type Boolean) (SweepResult :type "HitResult Structure (by ref)"))
  ;[1 1 1] Kill player on contact
  (bind _asbp_hero (cast `/Game/SHMUP_starter/Blueprints/Ship/BP_Hero` OtherActor))
  (`/Game/SHMUP_starter/Blueprints/Ship/BP_Hero.Die` :`self` _asbp_hero))

(event `self.TurretGun.OnComponentBeginOverlap`
  (params (OverlappedComponent :type "PrimitiveComponent Object Reference") (OtherActor :type "Actor Object Reference") (OtherComp :type "PrimitiveComponent Object Reference") (OtherBodyIndex :type Integer) (bFromSweep :type Boolean) (SweepResult :type "HitResult Structure (by ref)"))
  ;[1 1 1] Kill player on contact
  (bind _asbp_hero (cast `/Game/SHMUP_starter/Blueprints/Ship/BP_Hero` OtherActor))
  (`/Game/SHMUP_starter/Blueprints/Ship/BP_Hero.Die` :`self` _asbp_hero))

(fn `UserConstructionScript`)