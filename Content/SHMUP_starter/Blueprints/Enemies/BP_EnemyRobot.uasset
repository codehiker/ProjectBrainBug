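; Robot enemy for the shoot-'em-up that descends in bursts, firing a penetrating bullet between moves.
; Chained timelines play its intro (sphere fly-in, mesh reveal, slide and rotation), then start a self-repeating, delay-driven attack loop.
; Tick handles the descent down to a height floor.
; Hero damage flashes a hit material; death explodes, awards score, and either spawns a pickup or, without one, advances the LevelManager phase.
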(event `self.ReceiveBeginPlay`
  ;[1 1 1] Initialization
  (bind _asbp_hero (cast `/Game/SHMUP_starter/Blueprints/Ship/BP_Hero` (`GameplayStatics.GetPlayerPawn` 0)))
  (set `self.HeroRef` _asbp_hero)
  (set `self.DefaultMat` (`PrimitiveComponent.GetMaterial` (`self.SkeletalMesh`) 0))
  (`self.Intro`))

(event `self.ReceiveTick`
  (params (DeltaSeconds :type "Float (single-precision)"))
  (bind (_returnvalue_x _returnvalue_y _returnvalue_z) (`KismetMathLibrary.BreakVector` (`self.K2_GetActorLocation`)))
  (bind _heroref (`self.HeroRef`))
  ;[1 1 1] Tick - animate the robot staying in place and moving down.
  (`/Engine/EditorBlueprintResources/StandardMacros.IsValid` _heroref
    (:`Is Valid`
      (`self.K2_AddActorWorldOffset` (`KismetMathLibrary.MakeVector` 0.0 (* (`/Game/SHMUP_starter/Blueprints/Ship/BP_Hero.CurrentSpeed` _heroref) (* -1.0 0.0) DeltaSeconds)) true)
      (if (and (>= _returnvalue_z -500.0) (`self.MovingDown?`))
        (`self.K2_AddActorWorldOffset` (`KismetMathLibrary.MakeVector` 0.0 0.0 (* DeltaSeconds -150.0)) true)))))

(event `/Game/SHMUP_starter/Blueprints/BP_iDamageable.TakeDamage`
  (params (Aggressor :type "Actor Object Reference") (Damage :type "Float (single-precision)"))
  ;[1 1 1] Take damage
  (cast `/Game/SHMUP_starter/Blueprints/Ship/BP_Hero` Aggressor)
  (`self.Flash`)
  (bind _output_get (set `self.Health` (- (`self.Health`) Damage)))
  (if (<= _output_get 0.0)
    (`self.Die`)))

(event `Die`
  ;[1 1 1] Die
  (`/Engine/EditorBlueprintResources/StandardMacros.DoOnce` false
    (:`Completed`
      (`GameplayStatics.SpawnEmitterAtLocation` "/Game/SHMUP_starter/Particles/P_Explosion.P_Explosion" (`self.K2_GetActorLocation`) (struct) (0.5 0.5 0.5))
      (`GameplayStatics.PlaySoundAtLocation` "/Game/SHMUP_starter/Audio/Cues/EnemyDeath_Cue.EnemyDeath_Cue" (`self.K2_GetActorLocation`) (struct) 1.0 1.0 0.0 null null null)
      (`/Game/SHMUP_starter/Blueprints/Ship/BP_Hero.AddScore` (`self.HeroRef`) (`self.Score`))
      (if (`self.Drop?`)
        (`|SpawnActorFromClass` "/Game/SHMUP_starter/Blueprints/Weapons/BP_PickUp.BP_PickUp_C" (`self.GetTransform`) "Undefined" "OverrideRootScale" null (`self.Drop`) null)
        (else
          (`/Game/SHMUP_starter/Blueprints/LevelStuff/BP_LevelManager.PhaseUp` (`self.LevelManager`))))
      (`self.K2_DestroyActor`))))

(event `Flash`
  ;[1 1 1] Damage flash
  (`PrimitiveComponent.SetMaterial` (`self.SkeletalMesh`) 0 "/Game/SHMUP_starter/Materials/MI_Hit.MI_Hit")
  (`KismetSystemLibrary.Delay` 0.3)
  (`PrimitiveComponent.SetMaterial` (`self.SkeletalMesh`) 0 (`self.DefaultMat`)))

(event `StartAttack`
  ;[1 1 1] Commence attack
  (set `self.MovingDown?` true)
  (`KismetSystemLibrary.Delay` 1.3)
  (set `self.MovingDown?` false)
  (`KismetSystemLibrary.Delay` 0.2)
  (`self.Shoot`)
  (`self.StartAttack`))

(event `Shoot`
  ;[1 1 1] Firing
  (`self.ShootBullet`)
  (`SkeletalMeshComponent.PlayAnimation` (`self.SkeletalMesh`) "/Game/SHMUP_starter/Mannequin/Animations/A_Mech_Fire.A_Mech_Fire" false)
  (`KismetSystemLibrary.Delay` 0.35)
  (`SkeletalMeshComponent.PlayAnimation` (`self.SkeletalMesh`) "/Game/SHMUP_starter/Mannequin/Animations/A_Mech_Idle.A_Mech_Idle" false))

(event `ShootBullet`
  ;[1 1 1] Firing
  (`|SpawnActorFromClass` "/Game/SHMUP_starter/Blueprints/Weapons/BP_EnemyBullet.BP_EnemyBullet_C" (`SceneComponent.K2_GetComponentToWorld` (`self.Arrow`)) "Undefined" "OverrideRootScale" null 15.0 4000.0 true null))

(event `Intro`
  (bind _sphere (`self.Sphere`))
  ;[1 1 1] Intro animation
  (bind (_direction _movement) (`Timeline|Timeline_2` :!via `PlayFromStart`)
    (:`Update`
      (`SceneComponent.K2_SetRelativeLocation` _sphere (`KismetMathLibrary.MakeVector` 10000.0 (`KismetMathLibrary.Lerp` 20000.0 0.0 _movement) 93.333) false false))
    (:`Finished`
      (`SceneComponent.SetVisibility` _sphere false false)
      (`SceneComponent.SetHiddenInGame` (`self.SkeletalMesh`) false true)
      (bind (_direction_2 _movement_2) (`Timeline|Timeline_0` :!via `PlayFromStart`)
        (:`Update`
          (`SceneComponent.K2_SetRelativeLocation` (`self.Scene`) (`KismetMathLibrary.MakeVector` (`KismetMathLibrary.Lerp` 10000.0 0.0 _movement_2) 0.0 93.333) false false))
        (:`Finished`
          (bind (_direction_3 _movement_3) (`Timeline|Timeline_1` :!via `PlayFromStart`)
            (:`Update`
              (bind _returnvalue (`KismetMathLibrary.Lerp` -90.0 0.0 _movement_3))
              (`SceneComponent.K2_SetRelativeRotation` (`self.Scene`) (`KismetMathLibrary.MakeRotator` _returnvalue 0.0 _returnvalue) false false))
            (:`Finished`
              (`self.StartAttack`))))))))

(fn `UserConstructionScript`)