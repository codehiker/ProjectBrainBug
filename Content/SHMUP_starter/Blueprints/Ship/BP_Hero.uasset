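; Player ship pawn for a shoot-'em-up, handling movement, weapons, power-ups and death, and spawning its camera and HUD.
; A recursive delay loop drives auto-fire, relayed to attached Force and Sentry weapons.
; Tick builds charge for a damage-scaled shot or, at full charge in Hyper mode, a timed boost followed by overheat cooldown.
; Non-camera hits destroy attachments and spend a life from the game instance or show game over; number keys spawn debug drop ships.
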(event `self.ReceiveBeginPlay`
  ;[1 1 1] Initialization
  (`|ExecutionSequence`
    (:`then_0`
      ;;[1 1 1] Set up the camera
      (bind _returnvalue (`|SpawnActorFromClass` "/Game/SHMUP_starter/Blueprints/Camera/BP_CameraSystem.BP_CameraSystem_C" (`self.GetTransform`) "Undefined" "OverrideRootScale" null self null))
      (bind _output_get (set `self.CameraSystem` _returnvalue))
      (`PlayerController.SetViewTargetWithBlend` (`GameplayStatics.GetPlayerController` 0) _output_get 0.0 "VTBlend_Linear" 0.0 false)
      ;;[1 1 1] Pull the lives remaining from the instance
      (bind _asbp_turbo_instance (cast `/Game/SHMUP_starter/Blueprints/BP_TurboInstance` (`GameplayStatics.GetGameInstance`)))
      (set `self.Lives` (`/Game/SHMUP_starter/Blueprints/BP_TurboInstance.CurrentLives` _asbp_turbo_instance))
      ;;[1 1 1] Set up the input and capture
      (`WidgetBlueprintLibrary.SetInputMode_GameOnly` (`GameplayStatics.GetPlayerController` 0)))
    (:`then_1`
      ;;[1 1 1] Start up the firing tick and re-zero the Hero ship
      (`self.ShootTick`)
      (`self.K2_SetActorLocation` (0.0 0.0 0.0)))
    (:`then_2`
      ;;[1 1 1] Create HUD and the level intro fade
      (bind _returnvalue_2 (`|CreateWidget` "/Game/SHMUP_starter/Blueprints/UI/UI_HUD.UI_HUD_C"))
      (bind _output_get_2 (set `self.HUD` _returnvalue_2))
      (`UserWidget.AddToViewport` _output_get_2 0)
      (bind _returnvalue_3 (`|CreateWidget` "/Game/SHMUP_starter/Blueprints/UI/UI_LevelStart.UI_LevelStart_C"))
      (`UserWidget.AddToViewport` _returnvalue_3 0))))

(event `InputAction|Pause` :paused true
  (params (Key :type "Key Structure"))
  ;[1 1 1] Pause
  (:`Pressed`
    (bind _isa (`/Engine/EditorBlueprintResources/StandardMacros.FlipFlop`)
      (:`A`
        _)
      (:`B`
        _))
    (`GameplayStatics.SetGamePaused` _isa)
    (if _isa
      (`self.StopBGM`)
      (else
        (`self.StartBGM`)))))

(event `self.ReceiveTick`
  (params (DeltaSeconds :type "Float (single-precision)"))
  ;[1 1 1] Tick - handles tilting and charge bar
  (`self.Charging`) ; Check for charge
  (`SceneComponent.K2_SetRelativeRotation` (`self.ShipMesh`) (`KismetMathLibrary.MakeRotator` 0.0 (`KismetMathLibrary.MapRangeClamped` (`self.UpMove`) -1.0 1.0 25.0 -25.0)) false false) ; Tilt the ship based on Y movement
)

(event `Key|Escape`
  (params (Key :type "Key Structure"))
  ;[1 1 1] Quit game
  (:`Pressed`
    (`KismetSystemLibrary.QuitGame` null "Quit")))

(event `Key|One`
  (params (Key :type "Key Structure"))
  ;[1 0.8214 0] Cheats - for debug
  (:`Pressed`
    (`/Game/SHMUP_starter/Blueprints/LevelStuff/BP_LevelManager.SpawnDropShip` (`self.LevelManager`) "NewEnumerator3")))

(event `Key|Three`
  (params (Key :type "Key Structure"))
  ;[1 0.8214 0] Cheats - for debug
  (:`Pressed`
    (`/Game/SHMUP_starter/Blueprints/LevelStuff/BP_LevelManager.SpawnDropShip` (`self.LevelManager`) "NewEnumerator7")))

(event `InputAxis|MoveUp`
  (params (AxisValue :type "Float (single-precision)"))
  ;[1 1 1] Movement
  (if (not (`self.Dead?`))
    (bind _output_get (set `self.UpMove` AxisValue)) ; Capture for tilting
    (`self.AddMovementInput` (0.0 0.0 1.0) _output_get)))

(event `InputAxis|MoveRight`
  (params (AxisValue :type "Float (single-precision)"))
  ;[1 1 1] Movement
  (if (not (`self.Dead?`))
    (`self.AddMovementInput` (0.0 1.0 0.0) AxisValue)))

(event `Key|Two`
  (params (Key :type "Key Structure"))
  ;[1 0.8214 0] Cheats - for debug
  (:`Pressed`
    (`/Game/SHMUP_starter/Blueprints/LevelStuff/BP_LevelManager.SpawnDropShip` (`self.LevelManager`) "NewEnumerator6")))

(event `Key|Four`
  (params (Key :type "Key Structure"))
  ;[1 0.8214 0] Cheats - for debug
  (:`Pressed`
    (`/Game/SHMUP_starter/Blueprints/LevelStuff/BP_LevelManager.SpawnDropShip` (`self.LevelManager`) "NewEnumerator8")))

(event `self.ReceiveHit`
  (params (MyComp :type "PrimitiveComponent Object Reference") (Other :type "Actor Object Reference") (OtherComp :type "PrimitiveComponent Object Reference") (bSelfMoved :type Boolean) (HitLocation :type "Vector Structure") (HitNormal :type "Vector Structure") (NormalImpulse :type "Vector Structure") (Hit :type "HitResult Structure (by ref)"))
  ;[1 1 1] Death
  ;;[1 1 1] Check for hit, negate for camera blocking volumes.  Get normal for directional explosions.
  (if (not (== Other (`self.CameraSystem`)))
    (`self.Die` (`KismetMathLibrary.MakeRotFromZ` HitNormal))
    (set `self.Charging?` false)))

(event `Die`
  (params (HitRotation :type "Rotator Structure"))
  ;[1 1 1] Death
  ;;[1 1 1] Spawn death effects
  (`/Engine/EditorBlueprintResources/StandardMacros.DoOnce` false
    (:`Completed`
      (`|SpawnActorFromClass` "/Game/SHMUP_starter/Blueprints/FX/BP_Explosion.BP_Explosion_C" (`KismetMathLibrary.MakeTransform` (`self.K2_GetActorLocation`) HitRotation) "Undefined" "OverrideRootScale" null null) ; Spawn player explosion, rotate if needed
      (`GameplayStatics.PlaySoundAtLocation` "/Game/SHMUP_starter/Audio/Cues/Death_Cue.Death_Cue" (`self.K2_GetActorLocation`) (struct) 1.0 1.0 0.0 null null null) ; Play player death sound
      (set `self.Dead?` true)
      (`SceneComponent.SetHiddenInGame` (`self.ShipMesh`) true false) ; Hide player ship mesh
      (`self.StopBGM`) ; Turn level music off
      (`self.DestroyAttachments`)
      (`self.ReduceLives`))))

(event `ReduceLives`
  ;[1 1 1] Death
  ;;[1 1 1] Check remaining lives.  Game over if none.  Reduce and save to instance if there is stock.
  (if (<= (`self.Lives`) 0)
    (`self.GameOver`)
    (else
      (set `self.Lives` (- (`self.Lives`) 1))
      (bind _asbp_turbo_instance (cast `/Game/SHMUP_starter/Blueprints/BP_TurboInstance` (`GameplayStatics.GetGameInstance`)))
      (`/Game/SHMUP_starter/Blueprints/BP_TurboInstance.SaveStatus` _asbp_turbo_instance)
      (bind _returnvalue (`|CreateWidget` "/Game/SHMUP_starter/Blueprints/UI/UI_Dead.UI_Dead_C"))
      (`UserWidget.AddToViewport` _returnvalue 0))))

(event `GameOver`
  ;[1 1 1] Death
  ;;[1 1 1] Add game over to the screen - put game over logic here
  (bind _returnvalue (`|CreateWidget` "/Game/SHMUP_starter/Blueprints/UI/UI_GameOver.UI_GameOver_C"))
  (`UserWidget.AddToViewport` _returnvalue 0))

(event `StartCooldown`
  ;[1 1 1] Weapon systems
  ;;[1 1 1] Hyper cooldown timer
  (set `self.Cooldown` true)
  (set `self.HyperEnabled` false)
  (`AudioComponent.Play` (`self.CooldownAlarmSound`) 0.0)
  (`PrimitiveComponent.SetMaterial` (`self.ShipMesh`) 0 "/Game/SHMUP_starter/Materials/MI_Shmup_EM_4.MI_Shmup_EM_4") ; Change to overheat MAT
  (bind (_direction _cooldown) (`Timeline|CooldownTime` :!via `PlayFromStart`) ; Reduce charge back to 0
    (:`Update`
      (set `self.Charge` (* _cooldown 200.0)))
    (:`Finished`
      (set `self.Cooldown` false)
      (`PrimitiveComponent.SetMaterial` (`self.ShipMesh`) 0 "/Game/SHMUP_starter/Materials/MI_Shmup_1.MI_Shmup_1") ; Change back to normal MAT
      (`AudioComponent.Stop` (`self.CooldownAlarmSound`))
      (`self.ResetHyper`))))

(event `ShootTick`
  ;[1 1 1] Weapon systems
  ;;[1 1 1] Cycle gun system based on "Fire Rate."
  (if (not (`self.Dead?`))
    (if (`self.Shooting`)
      (`self.FireBullet`))
    (`KismetSystemLibrary.Delay` (`self.FireRate`))
    (`self.ShootTick`)))

(event `InputAction|Shoot`
  (params (Key :type "Key Structure"))
  ;[1 1 1] Weapon systems
  ;;[1 1 1] Enable shooting
  (:`Pressed`
    (if (not (or (`self.Charging?`) (`self.Dead?`)))
      (`self.FireBullet`)
      (set `self.Shooting` true)))
  (:`Released`
    (set `self.Shooting` false)))

(event `ResetHyper`
  ;[1 1 1] Weapon systems
  ;;[1 1 1] Shoot charged shot or start Hyper
  (goto _label :!via `Reset`))

(event `ChargeShot`
  (bind _charge (`self.Charge`))
  ;[1 1 1] Weapon systems
  ;;[1 1 1] Shoot charged shot or start Hyper
  (if (`self.Hyper`)
    (if (>= (`self.Charge`) 198.0)
      (`/Engine/EditorBlueprintResources/StandardMacros.DoOnce` false :!label _label
        (:`Completed`
          (set `self.HyperEnabled` true)
          (`KismetSystemLibrary.K2_SetTimer` null "StartCooldown" (`self.HyperDuration`)) ; Trigger cooldown after hyper duration
          (`GameplayStatics.SpawnEmitterAttached` "/Game/SHMUP_starter/Particles/P_HyperStart.P_HyperStart" (`self.ParticleDir`) "None" (0.0 0.0 0.0) (struct :`Pitch` -90.0) (1.0 1.0 1.0) "SnapToTarget") ; Hyper start effect
          (`GameplayStatics.PlaySoundAtLocation` "/Game/SHMUP_starter/Audio/Cues/HyperStart_Cue.HyperStart_Cue" (`self.K2_GetActorLocation`) (struct) 1.0 1.0 0.0 null null null)))
      (else
        (`|SpawnActorFromClass` "/Game/SHMUP_starter/Blueprints/Weapons/BP_Bullet.BP_Bullet_C" (`SceneComponent.K2_GetComponentToWorld` (`self.ParticleDir`)) "Undefined" "OverrideRootScale" null (+ (* (/ _charge 200.0) 23.0) 2.0) self (select `bool` (`self.Cooldown`) :`false` _charge :`true` 1.0) true false null :!label _label_2)
        (`GameplayStatics.PlaySoundAtLocation` (select `bool` (>= (`self.Charge`) 100.0) :`false` "/Game/SHMUP_starter/Audio/Cues/RegularShot_Cue.RegularShot_Cue" :`true` "/Game/SHMUP_starter/Audio/Cues/HyperShot_Cue.HyperShot_Cue" :!type "SoundBase Object Reference") (`self.K2_GetActorLocation`) (struct) 1.0 1.0 0.0 null null null)
        (set `self.Charge` 0.0)))
    (else
      (goto _label_2))))

(event `InputAction|HyperToggle`
  (params (Key :type "Key Structure"))
  ;[1 1 1] Weapon systems
  ;;[1 1 1] Switch to Hyper or Beam weapon
  (:`Pressed`
    (if (not (or (`self.HyperEnabled`) (`self.Cooldown`)))
      (bind _isa (`/Engine/EditorBlueprintResources/StandardMacros.FlipFlop`)
        (:`A`
          _)
        (:`B`
          _))
      (set `self.Hyper` _isa)
      (set `self.Charge` 0.0)
      (`GameplayStatics.PlaySound2D` "/Game/SHMUP_starter/Audio/Cues/HyperToggle_Cue.HyperToggle_Cue" 1.0 1.0 0.0 null null))))

(event `InputAction|Charge`
  (params (Key :type "Key Structure"))
  (bind _chargesound (`self.ChargeSound`))
  (bind _chargefx (`self.ChargeFX`))
  ;[1 1 1] Weapon systems
  ;;[1 1 1] Charge the main weapon
  (:`Pressed`
    (if (`self.Dead?`)
      _
      (elif (or (`self.Cooldown`) (`self.HyperEnabled`))
        (set `self.Shooting` true)
        (else
          (set `self.Charging?` true)
          (`AudioComponent.Play` _chargesound 0.0)
          (`ActorComponent.SetActive` _chargefx true true)))))
  (:`Released`
    (if (not (`self.Dead?`))
      (set `self.Shooting` false)
      (set `self.Charging?` false)
      (`self.ChargeShot`)
      (`AudioComponent.Stop` _chargesound)
      (`ActorComponent.SetActive` _chargefx false false))))

(event `InputAction|Detach`
  (params (Key :type "Key Structure"))
  (bind _forceweapon (`self.ForceWeapon`))
  ;[1 1 1] Weapon systems
  ;;[1 1 1] Eject the main power-up
  (:`Pressed`
    (`/Engine/EditorBlueprintResources/StandardMacros.IsValid` _forceweapon
      (:`Is Valid`
        (`/Game/SHMUP_starter/Blueprints/Weapons/BP_ForceWeapon.Launch` _forceweapon)))))

(event `self.FrontColl.OnComponentBeginOverlap`
  (params (OverlappedComponent :type "PrimitiveComponent Object Reference") (OtherActor :type "Actor Object Reference") (OtherComp :type "PrimitiveComponent Object Reference") (OtherBodyIndex :type Integer) (bFromSweep :type Boolean) (SweepResult :type "HitResult Structure (by ref)"))
  ;[1 1 1] Power ups
  (bind _asbp_force_weapon (cast `/Game/SHMUP_starter/Blueprints/Weapons/BP_ForceWeapon` OtherActor))
  (bind _output_get (set `self.ForceWeapon` _asbp_force_weapon))
  (if (`/Game/SHMUP_starter/Blueprints/Weapons/BP_ForceWeapon.Attachable` _output_get)
    (`self.K2_AttachToComponent` _output_get (`self.ForceFront`) "None" "SnapToTarget" "SnapToTarget" "KeepRelative" true)
    (`/Game/SHMUP_starter/Blueprints/Weapons/BP_ForceWeapon.Attach` _output_get)))

(event `self.RearColl.OnComponentBeginOverlap`
  (params (OverlappedComponent :type "PrimitiveComponent Object Reference") (OtherActor :type "Actor Object Reference") (OtherComp :type "PrimitiveComponent Object Reference") (OtherBodyIndex :type Integer) (bFromSweep :type Boolean) (SweepResult :type "HitResult Structure (by ref)"))
  ;[1 1 1] Power ups
  (bind _asbp_force_weapon (cast `/Game/SHMUP_starter/Blueprints/Weapons/BP_ForceWeapon` OtherActor))
  (bind _output_get (set `self.ForceWeapon` _asbp_force_weapon))
  (if (`/Game/SHMUP_starter/Blueprints/Weapons/BP_ForceWeapon.Attachable` _output_get)
    (`self.K2_AttachToComponent` _output_get (`self.ForceBack`) "None" "SnapToTarget" "SnapToTarget" "KeepRelative" true)
    (`/Game/SHMUP_starter/Blueprints/Weapons/BP_ForceWeapon.Attach` _output_get)))

(event `SpeedUp`
  (bind _floatingpawnmovement (`self.FloatingPawnMovement`))
  (bind _maxspeed (`FloatingPawnMovement.MaxSpeed` _floatingpawnmovement))
  ;[1 1 1] Power ups
  (if (< _maxspeed (`self.MaximumSpeed`))
    (set `FloatingPawnMovement.MaxSpeed` (+ _maxspeed 200.0) _floatingpawnmovement)))

(event `AddScore`
  (params (Score :type Integer))
  ;[1 1 1] Score
  (set `self.Score` (+ Score (`self.Score`))))

(fn `DestroyAttachments`
  (bind _sentry (`self.Sentry`))
  (bind _forceweapon (`self.ForceWeapon`))
  (bind _secondsentry (`/Game/SHMUP_starter/Blueprints/Weapons/BP_Sentry.SecondSentry` _sentry))
  ;[1 1 1] Check for and destroy any existing attachments.
  (`/Engine/EditorBlueprintResources/StandardMacros.IsValid` _forceweapon
    (:`Is Valid`
      (`self.K2_DestroyActor` _forceweapon))
    (:`Is Not Valid`
      _))
  (`/Engine/EditorBlueprintResources/StandardMacros.IsValid` _sentry
    (:`Is Valid`
      (`/Engine/EditorBlueprintResources/StandardMacros.IsValid` _secondsentry
        (:`Is Valid`
          (`self.K2_DestroyActor` _secondsentry))
        (:`Is Not Valid`
          _))
      (`self.K2_DestroyActor` _sentry))
    (:`Is Not Valid`
      _))
  (return))

(fn `FireBullet`
  (bind _sentry (`self.Sentry`))
  (bind _forceweapon (`self.ForceWeapon`))
  (bind _hyperenabled (`self.HyperEnabled`))
  (bind (_returnvalue_location _returnvalue_rotation _returnvalue_scale) (`KismetMathLibrary.BreakTransform` (`SceneComponent.K2_GetComponentToWorld` (`self.ParticleDir`))))
  ;[1 1 1] Spawn Bullet.  Scale for Hyper attack.
  (`|SpawnActorFromClass` "/Game/SHMUP_starter/Blueprints/Weapons/BP_Bullet.BP_Bullet_C" (`KismetMathLibrary.MakeTransform` _returnvalue_location _returnvalue_rotation (select `bool` _hyperenabled :`false` _returnvalue_scale :`true` (5.0 5.0 5.0))) "Undefined" "OverrideRootScale" null (select `bool` _hyperenabled :`false` 1.0 :`true` 10.0 :!type "Float (single-precision)") self 0.0 false false null)
  ;[1 1 1] Bullet sound
  (`GameplayStatics.PlaySoundAtLocation` (select `bool` (`self.HyperEnabled`) :`false` "/Game/SHMUP_starter/Audio/Cues/RegularShot_Cue.RegularShot_Cue" :`true` "/Game/SHMUP_starter/Audio/Cues/HyperShot_Cue.HyperShot_Cue" :!type "SoundBase Object Reference") (`self.K2_GetActorLocation`) (struct) 1.0 1.0 0.0 null null null)
  ;[1 1 1] Fire on power-ups (if available).
  (`/Engine/EditorBlueprintResources/StandardMacros.IsValid` _forceweapon
    (:`Is Valid`
      (`/Game/SHMUP_starter/Blueprints/Weapons/BP_ForceWeapon.Fire` _forceweapon))
    (:`Is Not Valid`
      _))
  (`/Engine/EditorBlueprintResources/StandardMacros.IsValid` _sentry
    (:`Is Valid`
      (`/Game/SHMUP_starter/Blueprints/Weapons/BP_Sentry.Fire` _sentry))
    (:`Is Not Valid`
      _))
  (return))

(fn `UserConstructionScript`)