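; BP_Explosion is a short-lived explosion actor for the SHMUP starter game.
; On BeginPlay it caches the player's BP_Hero and destroys itself after a brief delay, which only runs if that cast succeeds.
; Each Tick it shifts along negative Y by the hero's CurrentSpeed scaled by delta time, so the explosion moves with the character's speed.
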(event `self.ReceiveBeginPlay`
  ;[1 1 1] Initialization
  (bind _asbp_hero (cast `/Game/SHMUP_starter/Blueprints/Ship/BP_Hero` (`GameplayStatics.GetPlayerPawn` 0)))
  (set `self.HeroRef` _asbp_hero)
  (`KismetSystemLibrary.Delay` 1.5)
  (`self.K2_DestroyActor`))

(event `self.ReceiveTick`
  (params (DeltaSeconds :type "Float (single-precision)"))
  (bind _heroref (`self.HeroRef`))
  ;[1 1 1] Move the explosion with the character speed
  (`/Engine/EditorBlueprintResources/StandardMacros.IsValid` _heroref
    (:`Is Valid`
      (`self.K2_AddActorWorldOffset` (`KismetMathLibrary.MakeVector` 0.0 (* DeltaSeconds (`/Game/SHMUP_starter/Blueprints/Ship/BP_Hero.CurrentSpeed` _heroref) -1.0))))))

(fn `UserConstructionScript`)