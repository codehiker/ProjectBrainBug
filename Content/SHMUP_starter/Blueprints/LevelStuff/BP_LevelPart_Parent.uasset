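; Parent Blueprint for scrolling, self-repeating level pieces in a shoot 'em up.
; Each tick it moves along Y at its own Speed scaled by the hero's CurrentSpeed, with MoveLeft setting direction.
; Crossing SpawnTrigger fires once, spawning a copy of its own class at the SpawnPosition offset unless the hero's LevelManager is Done.
; The old piece then destroys itself after RemoveTime either way.
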(event `self.ReceiveBeginPlay`
  ;[1 1 1] Initialization
  (bind _asbp_hero (cast `/Game/SHMUP_starter/Blueprints/Ship/BP_Hero` (`GameplayStatics.GetPlayerPawn` 0)))
  (set `self.HeroRef` _asbp_hero))

(event `self.ReceiveTick`
  (params (DeltaSeconds :type "Float (single-precision)"))
  (bind (_returnvalue_x _returnvalue_y _returnvalue_z) (`KismetMathLibrary.BreakVector` (`self.K2_GetActorLocation`)))
  (bind (_returnvalue_x_2 _returnvalue_y_2) (`KismetMathLibrary.BreakVector` (`self.K2_GetActorLocation`)))
  (bind _heroref (`self.HeroRef`))
  ;[1 1 1] Move based on ship "speed"
  (`/Engine/EditorBlueprintResources/StandardMacros.IsValid` _heroref
    (:`Is Valid`
      (`self.K2_AddActorWorldOffset` (`KismetMathLibrary.MakeVector` 0.0 (* DeltaSeconds (`/Game/SHMUP_starter/Blueprints/Ship/BP_Hero.CurrentSpeed` _heroref) (* (select `bool` (`self.MoveLeft?`) :`false` 1.0 :`true` -1.0 :!type "Float (single-precision)") (`self.Speed`)))))
      ;[1 1 1] Trigger on position (SpawnTrigger)
      (if (<= _returnvalue_y_2 (`self.SpawnTrigger`))
        (`/Engine/EditorBlueprintResources/StandardMacros.DoOnce` false
          (:`Completed`
            ;[1 1 1] Check section "done" status, if not done - spawn (SpawnPosition), then destroy offscreen (RemoveTime)
            (if (not (`/Game/SHMUP_starter/Blueprints/LevelStuff/BP_LevelManager.Done` (`/Game/SHMUP_starter/Blueprints/Ship/BP_Hero.LevelManager` (`self.HeroRef`))))
              (`|SpawnActorFromClass` (`GameplayStatics.GetObjectClass` self) (`KismetMathLibrary.MakeTransform` (`KismetMathLibrary.MakeVector` _returnvalue_x (+ _returnvalue_y (`self.SpawnPosition`)) _returnvalue_z)) "Undefined" "OverrideRootScale" null null))
            (`KismetSystemLibrary.Delay` (`self.RemoveTime`))
            (`self.K2_DestroyActor`)))))))

(fn `UserConstructionScript`)