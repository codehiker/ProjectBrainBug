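; BP_Bullet_ForceLvl3 is a penetrating shoot-'em-up projectile, by its name the level 3 Force shot.
; Capsule overlaps send a damage message with the Aggressor and Damage to the other actor without destroying the bullet, which expires on a short timer after spawning.
; The construction script gives both cylinder meshes dynamic bullet materials, tinted magenta or blue by the ColorFlip switch.
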(event `self.ReceiveBeginPlay`
  ;[1 1 1] Destroy after 3 seconds
  (`KismetSystemLibrary.Delay` 3.0)
  (`self.K2_DestroyActor`))

(event `self.Capsule.OnComponentBeginOverlap`
  (params (OverlappedComponent :type "PrimitiveComponent Object Reference") (OtherActor :type "Actor Object Reference") (OtherComp :type "PrimitiveComponent Object Reference") (OtherBodyIndex :type Integer) (bFromSweep :type Boolean) (SweepResult :type "HitResult Structure (by ref)"))
  ;[1 1 1] Deal damage and penetrate
  (message `/Game/SHMUP_starter/Blueprints/BP_iDamageable.TakeDamage` OtherActor (`self.Aggressor`) (`self.Damage`)))

(fn `UserConstructionScript`
  ;[1 1 1] Set color of bullet
  (set `self.Color` (select `bool` (`self.ColorFlip`) :`false` (struct :`B` 1.0 :`A` 1.0) :`true` (struct :`R` 1.0 :`B` 1.0 :`A` 1.0) :!type "LinearColor Structure"))
  (bind _returnvalue (`PrimitiveComponent.CreateDynamicMaterialInstance` (`self.Cylinder`) 0 "/Game/SHMUP_starter/Materials/MI_Bullet.MI_Bullet" "None"))
  (`MaterialInstanceDynamic.SetVectorParameterValue` _returnvalue "Color" (`self.Color`))
  (bind _returnvalue_2 (`PrimitiveComponent.CreateDynamicMaterialInstance` (`self.Cylinder1`) 0 "/Game/SHMUP_starter/Materials/MI_Bullet.MI_Bullet" "None"))
  (`MaterialInstanceDynamic.SetVectorParameterValue` _returnvalue_2 "Color" (`self.Color`)))