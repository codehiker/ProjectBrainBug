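; BP_PickUp is a shoot 'em up power-up that grants the hero a force weapon, extra life, sentry or speed boost.
; It spins and scrolls along Y against the hero's current speed, showing a type icon set in the construction script.
; On hero overlap it plays a sound, switches on PickUpType and destroys itself.
; Force weapon and sentry pickups level up an existing instance or spawn one, with the sentry attached to the hero.
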(event `self.ReceiveBeginPlay`
  ;[1 1 1] Initialization
  (bind _asbp_hero (cast `/Game/SHMUP_starter/Blueprints/Ship/BP_Hero` (`GameplayStatics.GetPlayerPawn` 0)))
  (set `self.HeroRef` _asbp_hero))

(event `self.ReceiveTick`
  (params (DeltaSeconds :type "Float (single-precision)"))
  (bind _heroref (`self.HeroRef`))
  ;[1 1 1] Tick - rotate and move with player speed
  (`SceneComponent.K2_AddLocalRotation` (`self.Mesh`) (`/Game/SHMUP_starter/Blueprints/BP_SHMUP_MacroLibrary.RotationFI` (struct :`Yaw` 100.0)) false false)
  (`/Engine/EditorBlueprintResources/StandardMacros.IsValid` _heroref
    (:`Is Valid`
      (`self.K2_AddActorWorldOffset` (`KismetMathLibrary.MakeVector` 0.0 (* (`GameplayStatics.GetWorldDeltaSeconds`) (`/Game/SHMUP_starter/Blueprints/Ship/BP_Hero.CurrentSpeed` _heroref) -1.0))))))

(event `self.ReceiveActorBeginOverlap`
  (params (OtherActor :type "Actor Object Reference"))
  (bind _heroref (`self.HeroRef`))
  (bind _heroref_2 (`self.HeroRef`))
  (bind _sentry (`/Game/SHMUP_starter/Blueprints/Ship/BP_Hero.Sentry` (`self.HeroRef`)))
  (bind _forceweapon (`/Game/SHMUP_starter/Blueprints/Ship/BP_Hero.ForceWeapon` (`self.HeroRef`)))
  ;[1 1 1] Pick up and decide
  (cast `/Game/SHMUP_starter/Blueprints/Ship/BP_Hero` OtherActor)
  (`GameplayStatics.PlaySoundAtLocation` "/Game/SHMUP_starter/Audio/Cues/PickUp_Cue.PickUp_Cue" (`self.K2_GetActorLocation`) (struct) 1.0 1.0 0.0 null null null)
  (switch `/Game/SHMUP_starter/Blueprints/Enums/Enum_PickUpType` (`self.PickUpType`)
    (:`NewEnumerator3`
      ;[1 1 1] Add power-up or level existing
      (`/Engine/EditorBlueprintResources/StandardMacros.IsValid` _forceweapon
        (:`Is Valid`
          (`/Game/SHMUP_starter/Blueprints/Weapons/BP_ForceWeapon.LevelUp` _forceweapon))
        (:`Is Not Valid`
          (`|SpawnActorFromClass` "/Game/SHMUP_starter/Blueprints/Weapons/BP_ForceWeapon.BP_ForceWeapon_C" (`KismetMathLibrary.MakeTransform` (0.0 -500.0 0.0)) "AdjustIfPossibleButAlwaysSpawn" "OverrideRootScale" null null)))
      (`self.K2_DestroyActor`))
    (:`NewEnumerator6`
      ;[1 1 1] Add extra life
      (set `/Game/SHMUP_starter/Blueprints/Ship/BP_Hero.Lives` (+ (`/Game/SHMUP_starter/Blueprints/Ship/BP_Hero.Lives` _heroref_2) 1) _heroref_2)
      (`GameplayStatics.PlaySound2D` "/Game/SHMUP_starter/Audio/Cues/ExtraLife_Cue.ExtraLife_Cue" 1.0 1.0 0.0 null null)
      (`self.K2_DestroyActor`))
    (:`NewEnumerator7`
      ;[1 1 1] Add sentry or level up existing
      (`/Engine/EditorBlueprintResources/StandardMacros.IsValid` _sentry
        (:`Is Valid`
          (`/Game/SHMUP_starter/Blueprints/Weapons/BP_Sentry.LevelUp` _sentry))
        (:`Is Not Valid`
          (bind _returnvalue (`|SpawnActorFromClass` "/Game/SHMUP_starter/Blueprints/Weapons/BP_Sentry.BP_Sentry_C" (`KismetMathLibrary.MakeTransform` (0.0 0.0 0.0)) "AdjustIfPossibleButAlwaysSpawn" "OverrideRootScale" null _heroref null))
          (bind _output_get (set `/Game/SHMUP_starter/Blueprints/Ship/BP_Hero.Sentry` _returnvalue _heroref))
          (`self.K2_AttachToActor` _output_get _heroref "None" "SnapToTarget" "SnapToTarget" "KeepRelative" true)))
      (`self.K2_DestroyActor`))
    (:`NewEnumerator8`
      ;[1 1 1] Increase speed
      (`/Game/SHMUP_starter/Blueprints/Ship/BP_Hero.SpeedUp` (`self.HeroRef`))
      (`self.K2_DestroyActor`))))

(fn `UserConstructionScript`
  (locals (Icon :type Text))
  ;[1 1 1] Set symbol inside power-up
  (bind _output_get (set `local.Icon` (select `/Game/SHMUP_starter/Blueprints/Enums/Enum_PickUpType` (`self.PickUpType`) :`NewEnumerator3` "G" :`NewEnumerator6` "+" :`NewEnumerator7` "S" :`NewEnumerator8` ">" :!type "Text")))
  (`TextRenderComponent.K2_SetText` (`self.TextRender`) _output_get))