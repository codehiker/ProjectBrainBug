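; Detachable Force weapon pod for the SHMUP hero, which flies in on spawn and registers itself with BP_Hero.
; While detached, Tick steers it toward the player at distance-scaled speed and nudges it back inside screen bounds.
; Launch ejects it via timeline when attached, otherwise recalls it faster.
; Fire spawns more bullets as it levels up to three, while a self-repeating DamagePulse hurts overlapping actors.
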(event `self.ReceiveBeginPlay`
  ;[1 1 1] Initialization
  (bind _asbp_hero (cast `/Game/SHMUP_starter/Blueprints/Ship/BP_Hero` (`GameplayStatics.GetPlayerPawn` 0)))
  (bind _output_get (set `self.Hero` _asbp_hero))
  (set `/Game/SHMUP_starter/Blueprints/Ship/BP_Hero.ForceWeapon` self _output_get)
  (`self.K2_SetActorRotation` (struct :`Yaw` 90.0))
  (`self.DamagePulse`)
  (bind (_direction _location) (`Timeline|FlyIn` :!via `PlayFromStart`)
    (:`Update`
      (`self.K2_SetActorLocation` (`KismetMathLibrary.MakeVector` 0.0 (`KismetMathLibrary.Lerp` -2000.0 -1000.0 _location))))))

(event `self.ReceiveTick`
  (params (DeltaSeconds :type "Float (single-precision)"))
  (bind _returnvalue (`self.K2_GetActorLocation`))
  (bind (_returnvalue_x _returnvalue_y) (`KismetMathLibrary.BreakVector` (`self.K2_GetActorLocation`)))
  (bind (_returnvalue_x_2 _returnvalue_y_2) (`KismetMathLibrary.BreakVector` (`self.K2_GetActorLocation`)))
  (bind _returnmultiplier (`self.ReturnMultiplier`))
  (bind _returnvalue_2 (`self.K2_GetActorLocation` (`self.Hero`)))
  (bind _returnvalue_3 (`KismetMathLibrary.Vector_Distance` _returnvalue_2 _returnvalue))
  (bind (_returnvalue_x_3 _returnvalue_y_3 _returnvalue_z) (`KismetMathLibrary.BreakVector` (* (`KismetMathLibrary.GetForwardVector` (`KismetMathLibrary.FindLookAtRotation` _returnvalue _returnvalue_2)) (`KismetMathLibrary.MapRangeClamped` _returnvalue_3 150.0 800.0 (`/Game/SHMUP_starter/Blueprints/BP_SHMUP_MacroLibrary.FloatFI` 100.0) (`/Game/SHMUP_starter/Blueprints/BP_SHMUP_MacroLibrary.FloatFI` 400.0)))))
  ;[1 1 1] Tick
  ;;[1 1 1] Spin mesh
  (`SceneComponent.K2_AddLocalRotation` (`self.Mesh`) (`/Game/SHMUP_starter/Blueprints/BP_SHMUP_MacroLibrary.RotationFI` (struct :`Pitch` 100.0)) false false)
  ;;[1 1 1] Travel back onto screen
  (if (`self.Attached?`)
    _
    (elif (<= _returnvalue_y_2 -1300.0)
      (`self.K2_AddActorWorldOffset` (`KismetMathLibrary.MakeVector` 0.0 (`/Game/SHMUP_starter/Blueprints/BP_SHMUP_MacroLibrary.FloatFI` 1500.0)) true)
      (elif (>= _returnvalue_y 1300.0)
        (`self.K2_AddActorWorldOffset` (`KismetMathLibrary.MakeVector` 0.0 (`/Game/SHMUP_starter/Blueprints/BP_SHMUP_MacroLibrary.FloatFI` -1500.0)) true)
        (else
          ;;[1 1 1] Travel back towards player
          (if (> _returnvalue_3 150.0)
            (`self.K2_AddActorWorldOffset` (`KismetMathLibrary.MakeVector` 0.0 (* _returnvalue_y_3 _returnmultiplier) (* _returnvalue_z _returnmultiplier)) true)))))))

(event `Launch`
  ;[1 1 1] Launch the power-up in the direction it is facing
  (if (`self.Attached?`)
    (set `self.Attachable` false)
    (set `self.Attached?` false)
    (`self.K2_DetachFromActor` "KeepWorld" "KeepWorld")
    (`GameplayStatics.PlaySoundAtLocation` "/Game/SHMUP_starter/Audio/Cues/Launch_Cue.Launch_Cue" (`self.K2_GetActorLocation`) (struct) 1.0 1.0 0.0 null null null)
    (bind (_direction _location) (`Timeline|Eject` :!via `PlayFromStart`)
      (:`Update`
        (`self.K2_AddActorLocalOffset` (`KismetMathLibrary.MakeVector` (* _location (`/Game/SHMUP_starter/Blueprints/BP_SHMUP_MacroLibrary.FloatFI` (`self.LaunchVelocity`)))) true))
      (:`Finished`
        (set `self.Attachable` true)))
    (else
      (`self.Recall`))))

(event `Recall`
  ;[1 1 1] Recall power-up
  (set `self.Attachable` true)
  (set `self.ReturnMultiplier` 6.0)
  (`GameplayStatics.PlaySoundAtLocation` "/Game/SHMUP_starter/Audio/Cues/Recall_Cue.Recall_Cue" (`self.K2_GetActorLocation`) (struct) 1.0 1.0 0.0 null null null))

(event `Fire`
  ;[1 1 1] Fire weapon - level up differences
  (`|ExecutionSequence`
    (:`then_0`
      (`|SpawnActorFromClass` "/Game/SHMUP_starter/Blueprints/Weapons/BP_Bullet_Force.BP_Bullet_Force_C" (`SceneComponent.K2_GetComponentToWorld` (`self.FireLoc1`)) "Undefined" "OverrideRootScale" null (`self.BaseDamage`) (`self.Hero`) 0.0 false false null)
      (`|SpawnActorFromClass` "/Game/SHMUP_starter/Blueprints/Weapons/BP_Bullet_Force.BP_Bullet_Force_C" (`SceneComponent.K2_GetComponentToWorld` (`self.FireLoc2`)) "Undefined" "OverrideRootScale" null (`self.BaseDamage`) (`self.Hero`) 0.0 false false null))
    (:`then_1`
      (if (> (`self.Level`) 1)
        (`|SpawnActorFromClass` "/Game/SHMUP_starter/Blueprints/Weapons/BP_Bullet_Force.BP_Bullet_Force_C" (`SceneComponent.K2_GetComponentToWorld` (`self.FireLoc3`)) "Undefined" "OverrideRootScale" null (`self.BaseDamage`) (`self.Hero`) 0.0 false false null)
        (`|SpawnActorFromClass` "/Game/SHMUP_starter/Blueprints/Weapons/BP_Bullet_Force.BP_Bullet_Force_C" (`SceneComponent.K2_GetComponentToWorld` (`self.FireLoc4`)) "Undefined" "OverrideRootScale" null (`self.BaseDamage`) (`self.Hero`) 0.0 false false null)))
    (:`then_2`
      (if (> (`self.Level`) 2)
        (bind _isa (`/Engine/EditorBlueprintResources/StandardMacros.FlipFlop`) ; Alternate colors
          (:`A`
            _)
          (:`B`
            _))
        (`|SpawnActorFromClass` "/Game/SHMUP_starter/Blueprints/Weapons/BP_Bullet_ForceLvl3.BP_Bullet_ForceLvl3_C" (`SceneComponent.K2_GetComponentToWorld` (`self.FireLoc5`)) "Undefined" "OverrideRootScale" null (`self.BaseDamage`) (`self.Hero`) _isa null)))))

(event `LevelUp`
  ;[1 1 1] Level up weapon
  (if (< (`self.Level`) 3)
    (set `self.Level` (+ (`self.Level`) 1))))

(event `DamagePulse`
  ;[1 1 1] Damage enemies on collision
  (for _array_element (`PrimitiveComponent.GetOverlappingActors` (`self.Collision`) null)
    (message `/Game/SHMUP_starter/Blueprints/BP_iDamageable.TakeDamage` _array_element (`self.Hero`) 5.0))
  (`KismetSystemLibrary.Delay` 0.1)
  (`self.DamagePulse`))

(event `Attach`
  ;[1 1 1] Attached to player ship
  (set `self.Attached?` true)
  (`GameplayStatics.PlaySoundAtLocation` "/Game/SHMUP_starter/Audio/Cues/Attach_Cue.Attach_Cue" (`self.K2_GetActorLocation`) (struct) 1.0 1.0 0.0 null null null)
  (set `self.ReturnMultiplier` 1.0))

(fn `UserConstructionScript`)