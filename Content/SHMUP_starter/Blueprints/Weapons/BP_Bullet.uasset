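; BP_Bullet is a projectile for a SHMUP starter that damages actors it overlaps and expires after three seconds.
; Its construction script tints the mesh through a dynamic material instance and scales charged shots by a clamped ShotCharge.
; On overlap it sends TakeDamageMessage with the aggressor and damage, then destroys itself.
; Penetrator or sufficiently charged shots delay that destruction, so they pass through targets.
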(event `self.ReceiveBeginPlay`
  ;[1 1 1] Destroy after 3 seconds
  (`KismetSystemLibrary.Delay` 3.0)
  (`self.K2_DestroyActor`))

(event `self.Sphere1.OnComponentBeginOverlap`
  (params (OverlappedComponent :type "PrimitiveComponent Object Reference") (OtherActor :type "Actor Object Reference") (OtherComp :type "PrimitiveComponent Object Reference") (OtherBodyIndex :type Integer) (bFromSweep :type Boolean) (SweepResult :type "HitResult Structure (by ref)"))
  ;[1 1 1] Deal damage and destroy on contact or penetrate when 1 full bar of charge
  (message `/Game/SHMUP_starter/Blueprints/BP_iDamageable.TakeDamage` OtherActor (`self.Aggressor`) (`self.Damage`))
  (if (or (>= (`self.ShotCharge`) 100.0) (`self.Penetrator`))
    (`KismetSystemLibrary.Delay` 3.0))
  (`self.K2_DestroyActor`))

(fn `UserConstructionScript`
  ;[1 1 1] Set color of bullet
  (bind _returnvalue (`PrimitiveComponent.CreateDynamicMaterialInstance` (`self.Sphere`) 0 "/Game/SHMUP_starter/Materials/MI_Bullet.MI_Bullet" "None"))
  (`MaterialInstanceDynamic.SetVectorParameterValue` _returnvalue "Color" (`self.Color`))
  ;[1 1 1] Scale if charged
  (if (`self.Charge?`)
    (`self.SetActorScale3D` (* (10.0 10.0 10.0) (`KismetMathLibrary.FClamp` (/ (`self.ShotCharge`) 200.0) 0.1)))))