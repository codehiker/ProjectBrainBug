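; BP_EnemyBullet is the enemy projectile in a shoot-'em-up, killing BP_Hero on overlap.
; Its construction script applies color through a dynamic material instance, sets scale and feeds Speed into ProjectileMovement.
; Contact with the hero, a force weapon or a sentry destroys it immediately unless Penetrator is set.
; Otherwise it passes through, with delayed destruction capping its lifetime at seven seconds.
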(event `self.ReceiveBeginPlay`
  ;[1 1 1] Destroy after 7 seconds
  (`KismetSystemLibrary.Delay` 7.0)
  (`self.K2_DestroyActor`))

(event `self.Sphere1.OnComponentBeginOverlap`
  (params (OverlappedComponent :type "PrimitiveComponent Object Reference") (OtherActor :type "Actor Object Reference") (OtherComp :type "PrimitiveComponent Object Reference") (OtherBodyIndex :type Integer) (bFromSweep :type Boolean) (SweepResult :type "HitResult Structure (by ref)"))
  ;[1 1 1] Destroy on contact or kill player.  Destroy on contact with sentry or power-up
  (bind _asbp_hero (cast `/Game/SHMUP_starter/Blueprints/Ship/BP_Hero` OtherActor)
    (:`then`
      (`/Game/SHMUP_starter/Blueprints/Ship/BP_Hero.Die` :`self` _asbp_hero)
      (if (`self.Penetrator`) :!label _label
        (`KismetSystemLibrary.Delay` 7.0)))
    (:`CastFailed`
      (cast `/Game/SHMUP_starter/Blueprints/Weapons/BP_ForceWeapon` OtherActor
        (:`then`
          (goto _label))
        (:`CastFailed`
          (cast `/Game/SHMUP_starter/Blueprints/Weapons/BP_Sentry` OtherActor
            (:`then`
              (goto _label))
            (:`CastFailed`
              (`KismetSystemLibrary.Delay` 7.0)))))))
  (`self.K2_DestroyActor`))

(fn `UserConstructionScript`
  (bind _projectilemovement (`self.ProjectileMovement`))
  (bind _speed (`self.Speed`))
  ;[1 1 1] Set bullet color
  (bind _returnvalue (`PrimitiveComponent.CreateDynamicMaterialInstance` (`self.Sphere`) 0 "/Game/SHMUP_starter/Materials/MI_Bullet.MI_Bullet" "None"))
  (`MaterialInstanceDynamic.SetVectorParameterValue` _returnvalue "Color" (`self.Color`))
  ;[1 1 1] Set scale
  (`self.SetActorScale3D` (* (1.0 1.0 1.0) (`self.Scale`)))
  ;[1 1 1] Set bullet speed
  (set `ProjectileMovementComponent.InitialSpeed` _speed _projectilemovement)
  (set `ProjectileMovementComponent.MaxSpeed` _speed _projectilemovement))