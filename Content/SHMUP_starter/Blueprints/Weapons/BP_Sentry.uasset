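; A sentry weapon for the hero in the shoot 'em up that spins continuously and upgrades through pickups.
; Tick rotates the mesh and arrow while pinning FireDirection to a fixed world rotation.
; Level 2 spawns and attaches a second copy of itself, flipped to an offset position.
; From level 3, Fire spawns hero-owned bullets along FireDirection and relays the call to the second sentry.
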(event `self.ReceiveTick`
  (params (DeltaSeconds :type "Float (single-precision)"))
  ;[1 1 1] Tick - handle rotation
  (`SceneComponent.K2_AddLocalRotation` (`self.Mesh`) (`/Game/SHMUP_starter/Blueprints/BP_SHMUP_MacroLibrary.RotationFI` (struct :`Pitch` 200.0)) false false)
  (`SceneComponent.K2_AddLocalRotation` (`self.Arrow`) (`/Game/SHMUP_starter/Blueprints/BP_SHMUP_MacroLibrary.RotationFI` (struct :`Roll` 150.0)) false false)
  (`SceneComponent.K2_SetWorldRotation` (`self.FireDirection`) (struct :`Yaw` 90.0) false false))

(event `LevelUp`
  ;[1 1 1] Level up on pick-up
  (bind _output_get (set `self.Level` (+ (`self.Level`) 1)))
  (switch `int` _output_get
    (:`2`
      (bind _returnvalue (`|SpawnActorFromClass` "BP_Sentry_C" (`KismetMathLibrary.MakeTransform` (0.0 0.0 0.0)) "Undefined" "OverrideRootScale" null (`self.Hero`) null))
      (bind _output_get_2 (set `self.SecondSentry` _returnvalue))
      (`self.K2_AttachToActor` _output_get_2 self "None" "SnapToTarget" "SnapToTarget" "KeepRelative" true)
      (`self.Flip` _output_get_2)
      (`SceneComponent.K2_SetRelativeRotation` :`self` (`self.Arrow`)))
    (:`3`
      (set `/Game/SHMUP_starter/Blueprints/Weapons/BP_Sentry.Level` 3 (`self.SecondSentry`)))))

(event `Flip`
  ;[1 1 1] Flip second sentry position
  (set `self.Secondary` true)
  (`SceneComponent.K2_SetRelativeRotation` :`self` (`self.Arrow`))
  (`SceneComponent.K2_SetRelativeLocation` (`self.Mesh`) (0.0 0.0 -300.0) false false))

(event `Fire`
  (bind _secondsentry (`self.SecondSentry`))
  (bind (_returnvalue_location _returnvalue_rotation) (`KismetMathLibrary.BreakTransform` (`SceneComponent.K2_GetComponentToWorld` (`self.FireDirection`))))
  ;[1 1 1] Fire projectile when leveled up
  (if (>= (`self.Level`) 3)
    (`|SpawnActorFromClass` "/Game/SHMUP_starter/Blueprints/Weapons/BP_Bullet.BP_Bullet_C" (`KismetMathLibrary.MakeTransform` _returnvalue_location _returnvalue_rotation) "Undefined" "OverrideRootScale" null 1.0 (`self.Hero`) 0.0 false false null)
    (`/Engine/EditorBlueprintResources/StandardMacros.IsValid` _secondsentry
      (:`Is Valid`
        (`self.Fire` _secondsentry)))))

(fn `UserConstructionScript`)