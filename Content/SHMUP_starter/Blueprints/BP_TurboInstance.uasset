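; BP_TurboInstance holds the player's lives, level and checkpoint for level transitions in the SHMUP starter game.
; SaveStatus casts the first player pawn to BP_Hero and copies those three values from it, stopping if the cast fails.
; GameOver resets the stored lives to a default and then calls SaveStatus, which overwrites that reset with the hero's current lives when the cast succeeds.
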(event `SaveStatus`
  ;[1 1 1] Set player values for level transition
  (bind _asbp_hero (cast `/Game/SHMUP_starter/Blueprints/Ship/BP_Hero` (`GameplayStatics.GetPlayerPawn` 0)))
  (set `self.CurrentLives` (`/Game/SHMUP_starter/Blueprints/Ship/BP_Hero.Lives` _asbp_hero))
  (set `self.CurrentLevel` (`/Game/SHMUP_starter/Blueprints/Ship/BP_Hero.CurrentLevel` _asbp_hero))
  (set `self.CurrentCheckpoint` (`/Game/SHMUP_starter/Blueprints/Ship/BP_Hero.CurrentCheckpoint` _asbp_hero)))

(event `GameOver`
  ;[1 1 1] Reset lives on game over
  (set `self.CurrentLives` 3)
  (`self.SaveStatus`))